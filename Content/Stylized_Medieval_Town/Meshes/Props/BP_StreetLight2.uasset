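; BP_StreetLight2 is a street light prop Blueprint that makes its point light flicker with random intensity and attenuation radius.
; Tick accumulates elapsed time and compares it to a threshold re-rolled each frame between the min and max flicker times.
; The timer is never reset, so once it passes the maximum, both light values are randomized every frame.
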(event EventBeginPlay)

(event Collision|EventActorBeginOverlap
  (params (OtherActor :type Actor%20Object%20Reference)))

(event EventTick
  (params (DeltaSeconds :type Float%20%28single-precision%29))
  (bind _pointlight (Variables|Default|GetPointLight))
  (bind _output_get (Variables|Default|Settimer (+ DeltaSeconds (Variables|Default|Gettimer))))
  (if (> _output_get (Math|Random|RandomFloatinRange (Variables|Default|GetminFlickerTime) (Variables|Default|GetmaxFlickerTime)))
    (Rendering|Components|Light|SetIntensity _pointlight (Math|Random|RandomFloatinRange (Variables|Default|GetminIntensity) (Variables|Default|GetmaxIntensity)))
    (Rendering|Lighting|SetAttenuationRadius _pointlight (Math|Random|RandomFloatinRange (Variables|Default|GetminAttenuationRadius) (Variables|Default|GetmaxAttenuationRadius)))))

(fn ConstructionScript)