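; BP_Target is the stealth game's target character, which patrols a list of points and can be hit by the player or escape.
; Tick starts each AIMoveTo leg behind a CanMove gate, then a successful move waits and advances the patrol index.
; Overlapping a trigger volume calls TargetLost on the player character.
; HitByPlayer ends the game with a win widget and camera fade, while an escape-widget event awaits external calls.
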(event Custom|HitByPlayer
  (params (Player :type BP%20Third%20Person%20Character%20Custom%20Object%20Reference))
  (Variables|/Game/StealthGame/Core/Characters/PlayerCharacter/BP_ThirdPersonCharacterCustom.BP_ThirdPersonCharacterCustom_C|SetbGameEnded Player true)
  (CallFunction|ShowYouWinWidget)
  (CameraFades|StartCameraFade :self (Game|GetPlayerCameraManager 0) :ToAlpha 1.0 :Duration 0.9 :bHoldWhenFinished true) ; Fade to black - duration is effected by the subsequent time dilation
)

(event Custom|ShowTargetEscapeWidget
  (UserInterface|Viewport|AddtoViewport (Variables|Default|GetTargetEscapeWidget) 0))

(event Custom|ShowYouWinWidget
  (UserInterface|Viewport|AddtoViewport (Variables|Default|GetYouWinWidget) 0))

(event Custom|GetNextPatrolTarget
  (if (> (+ (Variables|Default|GetCurrentIndex) 1) (Utilities|Array|Length (Variables|Default|GetPatrolTargetPoints)))
    (Variables|Default|SetCurrentIndex 0)
    (else
      (Variables|Default|SetCurrentIndex (+ (Variables|Default|GetCurrentIndex) 1)))))

(event Custom|MoveToNextTargetPoint
  (CallFunction|UpdateWalkSpeed (Variables|Default|GetPatrolSpeed))
  (Variables|Default|SetbCanMove false)
  (AI|AIMoveTo self "0, 0, 0" (Utilities|Array|Get(acopy) (Variables|Default|GetPatrolTargetPoints) (Variables|Default|GetCurrentIndex)) 1.0 false
    (:OnSuccess
      (Utilities|FlowControl|Delay (Variables|Default|GetPatrolDelay))
      (CallFunction|GetNextPatrolTarget)
      (Variables|Default|SetbCanMove true))))

(event EventBeginPlay
  ;[1 1 1] Add Widgets.
)

(event Collision|EventActorBeginOverlap
  (params (OtherActor :type Actor%20Object%20Reference))
  (Utilities|Casting|CastToTriggerVolume OtherActor)
  (bind _asbp_third_person_character_custom (Utilities|Casting|CastToBP_ThirdPersonCharacterCustom (Game|Player|GetPlayerPawn 0)))
  (Default|TargetLost _asbp_third_person_character_custom))

(event EventTick
  (params (DeltaSeconds :type Float%20%28single-precision%29))
  (if (Variables|Default|GetbCanMove)
    (CallFunction|MovetoNextTargetPoint)))

(fn ConstructionScript)

(fn UpdateWalkSpeed
  (params (NewWalkSpeed :type Float%20%28double-precision%29))
  (Variables|/Script/Engine.CharacterMovementComponent|SetMaxWalkSpeed (Variables|Character|GetCharacterMovement) NewWalkSpeed))