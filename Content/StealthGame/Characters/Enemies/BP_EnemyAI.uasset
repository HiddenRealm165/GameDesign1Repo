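; Stealth-game guard enemy that patrols, investigates noises, chases the player on sight, melees in range and can be temporarily stunned by player hits.
; Tick picks attack, chase, or one of three navigation modes (random, patrol points, guarding a pawn), gated by flags that AI MoveTo callbacks reset after delays.
; PawnSensing drives detection, with a looping timer clearing sight and toggling conflict audio.
; A montage notify fires the melee sphere trace.
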(event OnSeePawn(PawnSensing)
  (params (Pawn :type Pawn%20Object%20Reference))
  (if (Actor|ActorHasTag Pawn "Player")
    (Development|PrintString "Player Spotted")
    (Variables|Default|SetbPlayerVisible true)
    (Variables|Default|SetLastSeenTime (Utilities|Time|GetTimeSeconds))
    (bind _returnvalue (Utilities|Time|SetTimerbyFunctionName 0 "CheckLostSight" 0.5 true true))
    (Variables|Default|SetCheckLastSightHandler _returnvalue)
    (Default|EnterConflict (Variables|Default|GetAudioControllerRef))))

(event OnHearNoise(PawnSensing)
  (params (Instigator :type Pawn%20Object%20Reference) (Location :type Vector%20%28by%20ref%29 :default "0, 0, 0") (Volume :type Float%20%28single-precision%29))
  (if (not (Variables|Default|GetbPlayerVisible))
    (CallFunction|UpdateWalkSpeed (Variables|Default|GetPatrolSpeed))
    (Variables|Default|SetbCanPatrol false)
    (AI|AIMoveTo self Location 0 1e+01 false
      (:OnSuccess
        (Utilities|FlowControl|Delay (Variables|Default|GetPatrolDelay))
        (Variables|Default|SetbCanPatrol true)))))

(event Custom|HitByPlayer
  (params (Player :type BP%20Third%20Person%20Character%20Custom%20Object%20Reference))
  (Variables|Default|SetbStunned true)
  (Components|Movement|StopMovementImmediately (Variables|Character|GetCharacterMovement))
  (Variables|Default|SetbCanChase false)
  (Variables|Default|SetbCanPatrol false)
  (Variables|Default|SetbPlayerVisible false)
  (Class|NiagaraComponent|SetAsset (Variables|Default|GetNiagara) "/Game/StealthGame/Effects/Stun/NS_Stun.NS_Stun" true)
  (Utilities|FlowControl|Delay (Variables|Default|GetStunTime))
  (Variables|Default|SetbCanChase true)
  (Variables|Default|SetbCanPatrol true)
  (Class|NiagaraComponent|SetAsset (Variables|Default|GetNiagara) 0 true)
  (Variables|Default|SetbStunned false))

(event Custom|Attack
  (bind _mesh (Variables|Character|GetMesh))
  (bind _returnvalue (Transformation|GetSocketLocation _mesh "hand_r"))
  ;[0.15 0.15 0.15 0.5] Melee Attack
  (Utilities|FlowControl|DoOnce false
    (:Completed
      (bind _notifyname (Animation|Montage|PlayMontage (Variables|Character|GetMesh) "/Game/StealthGame/Characters/Enemies/AM_Attack_01.AM_Attack_01")
        (:OnCompleted
          (CallFunction|ResetAttack))
        (:OnNotifyBegin
          (switch name _notifyname
            (:AttackDamage
              (bind (_outhits _returnvalue_2) (Collision|MultiSphereTraceForObjects _returnvalue (+ _returnvalue (* (Transformation|GetActorForwardVector) (Variables|Default|GetMeleeTraceDistance))) (Variables|Default|GetMeleeTraceRadius) (Utilities|Array|MakeArray "ObjectTypeQuery3") false 0 "None"))
              (if _returnvalue_2
                (for _array_element _outhits
                  (bind _asbp_third_person_character_custom (Utilities|Casting|CastToBP_ThirdPersonCharacterCustom (.HitActor (Collision|BreakHitResult _array_element))))
                  (Default|HitbyGuard _asbp_third_person_character_custom))))))))))

(event Custom|GetNextPatrolTarget
  (Variables|Default|SetCurrentIndex (Math|Integer|%(Integer) (+ (Variables|Default|GetCurrentIndex) 1) (Utilities|Array|Length (Variables|Default|GetPatrolTargetPoints)))))

(event Custom|CheckLostSight
  (if (or (> (- (Utilities|Time|GetTimeSeconds) (Variables|Default|GetLastSeenTime)) (Variables|Default|GetSightTimeout)) (Variables|Default|GetbPlayerInAttackRange))
    (Variables|Default|SetbPlayerInAttackRange false)
    (Variables|Default|SetbPlayerVisible false)
    (Variables|Default|SetbCanChase true)
    (Utilities|Time|ClearandInvalidateTimerbyHandle (Variables|Default|GetCheckLastSightHandler))
    (Development|PrintString "Player Lost")
    (Default|ExitConflict (Variables|Default|GetAudioControllerRef))))

(event Custom|ResetAttack
  (bind _mesh (Variables|Character|GetMesh))
  (bind _returnvalue (Transformation|GetSocketLocation _mesh "hand_r"))
  ;[0.15 0.15 0.15 0.5] Melee Attack
  (Utilities|FlowControl|DoOnce false) ; enters at Reset
)

(event Custom|MoveToNextTargetPoint
  (CallFunction|UpdateWalkSpeed (Variables|Default|GetPatrolSpeed))
  (Variables|Default|SetbCanPatrol false)
  (AI|AIMoveTo self "0, 0, 0" (Utilities|Array|Get(acopy) (Variables|Default|GetPatrolTargetPoints) (Variables|Default|GetCurrentIndex)) 5.0 false
    (:OnSuccess
      (Utilities|FlowControl|Delay (Variables|Default|GetPatrolDelay))
      (CallFunction|GetNextPatrolTarget)
      (Variables|Default|SetbCanPatrol true))))

(event Custom|ChasePlayer
  (params (Pawn :type Pawn%20Object%20Reference))
  (CallFunction|UpdateWalkSpeed (Variables|Default|GetChaseSpeed))
  (Variables|Default|SetbCanPatrol false)
  (Variables|Default|SetbCanChase false)
  (AI|AIMoveTo self "0, 0, 0" (Game|GetPlayerController 0) 5e+01 true
    (:OnSuccess
      _)
    (:OnFail
      _))
  (Variables|Default|SetbPlayerVisible false)
  (Utilities|FlowControl|Delay (Variables|Default|GetChaseDelay))
  (Variables|Default|SetbCanPatrol true)
  (Variables|Default|SetbCanChase true))

(event Custom|GuardTarget
  (Variables|Default|SetbCanPatrol false)
  (if (> (Transformation|GetDistanceTo (Variables|Default|GetPawnToGuard) self) (Variables|Default|GetPreferedGuardDistance))
    (CallFunction|UpdateWalkSpeed (Variables|Default|GetChaseSpeed))
    (else
      (CallFunction|UpdateWalkSpeed (Variables|Default|GetPatrolSpeed))))
  (AI|AIMoveTo self (.RandomLocation (AI|Navigation|GetRandomReachablePointinRadius (Transformation|GetActorLocation (Variables|Default|GetPawnToGuard)) (Variables|Default|GetPreferedGuardDistance) 0 0)) 0 5.0 false
    (:OnSuccess
      (Utilities|FlowControl|Delay (Variables|Default|GetGuardDelay))
      (Variables|Default|SetbCanPatrol true))))

(event Custom|RandomPatrol
  (CallFunction|UpdateWalkSpeed (Variables|Default|GetPatrolSpeed))
  (Variables|Default|SetbCanPatrol false)
  (AI|AIMoveTo self (.RandomLocation (AI|Navigation|GetRandomReachablePointinRadius (Transformation|GetActorLocation) (Variables|Default|GetPatrolRadius) 0 0)) 0 5.0 false
    (:OnSuccess
      (Utilities|FlowControl|Delay (Variables|Default|GetPatrolDelay))
      (Variables|Default|SetbCanPatrol true))))

(event EventBeginPlay)

(event Collision|EventActorBeginOverlap
  (params (OtherActor :type Actor%20Object%20Reference))
  (if (Actor|ActorHasTag OtherActor "Player")
    (Variables|Default|SetbPlayerInAttackRange true)))

(event EventTick
  (params (DeltaSeconds :type Float%20%28single-precision%29))
  (if (not (Variables|Default|GetbStunned))
    (if (== (Utilities|Array|Length (Collision|GetOverlappingActors (Variables|Default|GetAttackRangeCollision) "/Game/StealthGame/Core/Characters/PlayerCharacter/BP_ThirdPersonCharacterCustom.BP_ThirdPersonCharacterCustom_C" :!class /Script/Engine.PrimitiveComponent)) 0)
      (Variables|Default|SetbPlayerInAttackRange false))
    (if (and (Variables|Default|GetbPlayerVisible) (Variables|Default|GetbPlayerInAttackRange))
      (Components|Movement|StopMovementImmediately (Variables|Character|GetCharacterMovement))
      (CallFunction|Attack)
      (elif (Variables|Default|GetbPlayerVisible)
        (if (Variables|Default|GetbCanChase)
          (CallFunction|ChasePlayer)
          (else
            (if (Variables|Default|GetbCanPatrol) :!label _label
              (switch Utilities|FlowControl|Switch|SwitchonE_NavigationType (Variables|Default|GetNavigationType)
                (:NewEnumerator0
                  (CallFunction|RandomPatrol))
                (:NewEnumerator1
                  (CallFunction|MovetoNextTargetPoint))
                (:NewEnumerator3
                  (CallFunction|GuardTarget))))))
        (else
          (goto _label))))))

(fn ConstructionScript)

(fn UpdateWalkSpeed
  (params (NewWalkSpeed :type Float%20%28double-precision%29))
  (Variables|/Script/Engine.CharacterMovementComponent|SetMaxWalkSpeed (Variables|Character|GetCharacterMovement) NewWalkSpeed))